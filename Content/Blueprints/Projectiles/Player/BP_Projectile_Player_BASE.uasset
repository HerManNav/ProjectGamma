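; Base Blueprint for player projectiles that removes them once they leave the screen horizontally.
; Tick, noted as running at a 0.05-second interval, calls DestroyIfOutsideTheViewport after the parent tick.
; That function projects the actor location to screen space through player controller 0 and destroys the actor when X falls outside the viewport width, ignoring the vertical axis.
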(event EventBeginPlay)

(event Collision|EventActorBeginOverlap
  (params (OtherActor :type Actor%20Object%20Reference)))

(event EventTick
  (params (DeltaSeconds :type Float%20%28single-precision%29))
  ;[1 1 1] Tick interval 0.05 secs!
  (|CallParentFunction DeltaSeconds)
  (CallFunction|DestroyifOutsidetheViewport))

(fn ConstructionScript
  (|CallParentFunction))

(fn DestroyifOutsidetheViewport
  (bind _returnvalue (Game|GetPlayerController 0))
  (bind _returnvalue_2 (Transformation|GetActorLocation))
  (bind _screenlocation (Class|PlayerController|ProjectWorldLocationtoScreen _returnvalue _returnvalue_2 false))
  (if (or (< (.x _screenlocation) 0.0) (> (.x _screenlocation) (.x (Viewport|GetViewportSize))))
    (Actor|DestroyActor)))