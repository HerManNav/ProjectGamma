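; BP_Player is the side-scrolling player character, with jump, dash, wall slide and charge shot.
; Shot hold time selects one of three projectiles, whose energy cost doubles as damage.
; A timeline drives the capsule-resizing dash, while a per-tick trace detects wall slides, which alter the physics volume's TerminalVelocity to control fall speed.
; Hits cause knockback, input lockout and flickering invincibility; defeat fades the camera and respawns through BP_PlayerGameMode.
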(event OnComponentBeginOverlap(CapsuleComponent)
  (params (OverlappedComponent :type Primitive%20Component%20Object%20Reference) (OtherActor :type Actor%20Object%20Reference) (OtherComp :type Primitive%20Component%20Object%20Reference) (OtherBodyIndex :type Integer) (bFromSweep :type Boolean) (SweepResult :type Hit%20Result%20Structure%20%28by%20ref%29))
  ;[1 1 1] Damage
  (CallFunction|ApplyDamageifEnemy OtherActor OtherComp))

(event Custom|Knockback
  (params (DamageCauser :type Actor%20Object%20Reference))
  ;[1 1 1] Damage
  (Variables|/Script/Engine.CharacterMovementComponent|SetFallingLateralFriction (Variables|Character|GetCharacterMovement) 0.0)
  (Character|LaunchCharacter (Math|Vector|MakeVector (* (|GetBackwardsDirection DamageCauser) (Variables|Damage|GetKnockbackVelocityHorizontal)) 0.0 (Variables|Damage|GetKnockbackVelocityVertical)) true true)
  (|ResetLateralFrictionToDefault))

(event Custom|OnCharacterDefeated
  (|RespawnSequence))

(event Custom|SetInvincible
  ;[1 1 1] Damage
  (Utilities|FlowControl|Sequence
    (:then_0
      (bind _flickeringtimer (|StartFlicking))
      (Collision|SetCollisionResponsetoChannel (Variables|Default|GetCapsuleComponent) "ECC_Pawn" "ECR_Ignore"))
    (:then_1
      (Utilities|FlowControl|Delay (Variables|Damage|GetInvincibilityDuration))
      (Utilities|Time|ClearandInvalidateTimerbyHandle _flickeringtimer)
      (Collision|SetCollisionResponsetoChannel (Variables|Default|GetCapsuleComponent) "ECC_Pawn" "ECR_Overlap")
      (Rendering|SetVisibility (Variables|Default|GetSprite) true false))))

(event Input|EnhancedActionEvents|EnhancedInputActionIA_Jump
  (params (ActionValue :type Boolean) (ElapsedSeconds :type Float%20%28double-precision%29) (TriggeredSeconds :type Float%20%28double-precision%29) (InputAction :type Input%20Action%20Object%20Reference :default "/Game/Input/IA_Jump.IA_Jump"))
  ;[1 1 1] Basic movement
  (:Started
    (if (Variables|WallSlide|GetIsWallSliding)
      (|WallSlidingJump)
      (else
        (Character|Jump)
        (Variables|Dash|SetIsDashing false))))
  (:Completed
    (Character|StopJumping)))

(event Input|EnhancedActionEvents|EnhancedInputActionIA_Dash
  (params (ActionValue :type Boolean) (ElapsedSeconds :type Float%20%28double-precision%29) (TriggeredSeconds :type Float%20%28double-precision%29) (InputAction :type Input%20Action%20Object%20Reference :default "/Game/Input/IA_Dash.IA_Dash"))
  ;[1 1 1] Dash
  (:Started
    (if (and (not (Variables|Dash|GetIsDashing)) (not (AI|Components|NavMovement|IsFalling (Variables|Character|GetCharacterMovement))))
      (|Dash))))

(event Input|EnhancedActionEvents|EnhancedInputActionIA_Shoot
  (params (ActionValue :type Boolean) (ElapsedSeconds :type Float%20%28double-precision%29) (TriggeredSeconds :type Float%20%28double-precision%29) (InputAction :type Input%20Action%20Object%20Reference :default "/Game/Input/IA_Shoot.IA_Shoot"))
  (bind _returnvalue (|CanShoot))
  ;[1 1 1] Shoot
  (:Started
    (if _returnvalue
      (Variables|Shoot|SetIsShooting true)))
  (:Ongoing
    (if _returnvalue
      (CallFunction|HandleChargingFlash ElapsedSeconds)
      (Utilities|FlowControl|RetriggerableDelay (Variables|Shoot|GetPostAimDuration))
      (Variables|Shoot|SetIsShooting false)))
  (:Completed
    (if _returnvalue
      (Utilities|FlowControl|Sequence
        (:then_0
          (Variables|Flash|PartialCharge|SetPartialChargeAlreadyFlashed false)
          (Variables|Flash|FullCharge|SetFullChargeAlreadyFlashed false))
        (:then_1
          (if (Variables|Shoot|GetHasBeenDamagedWhileCharging)
            (Variables|Shoot|SetHasBeenDamagedWhileCharging false)
            (else
              (|Shoot ElapsedSeconds))))))))

(event Input|EnhancedActionEvents|EnhancedInputActionIA_MoveRightLeft
  (params (ActionValue :type Float%20%28double-precision%29) (ElapsedSeconds :type Float%20%28double-precision%29) (TriggeredSeconds :type Float%20%28double-precision%29) (InputAction :type Input%20Action%20Object%20Reference :default "/Game/Input/IA_MoveRightLeft.IA_MoveRightLeft"))
  ;[1 1 1] Basic movement
  (Utilities|FlowControl|Sequence
    (:then_0
      (Variables|Movement|SetMovementAmountRightLeft (Math|Float|Absolute(Float) ActionValue)))
    (:then_1
      (Pawn|Input|AddMovementInput "1.000000,0.000000,0.000000" ActionValue false)
      (CallFunction|RotateXDirection ActionValue))
    (:then_2
      (if (and (Variables|Dash|GetIsDashing) (not (Math|Float|NearlyEqual(Float) ActionValue (Variables|Dash|GetDashDirection) 1e-06)))
        (CallFunction|StopDash)))))

(event Input|EnhancedActionEvents|EnhancedInputActionIA_MoveUpDown
  (params (ActionValue :type Float%20%28double-precision%29) (ElapsedSeconds :type Float%20%28double-precision%29) (TriggeredSeconds :type Float%20%28double-precision%29) (InputAction :type Input%20Action%20Object%20Reference :default "/Game/Input/IA_MoveUpDown.IA_MoveUpDown"))
  ;[1 1 1] Wall Sliding
  (if (|IsPressingDownWhileWallSliding ActionValue)
    (|IncreaseFallVelocity ActionValue)))

(event EventBeginPlay
  (|CallParentFunction)
  (EventDispatchers|BindEventtoCharacterDefeated (delegate Custom|OnCharacterDefeated))
  (|SaveOriginalValues)
  ;[1 1 1] This should be ALWAYS at the end of the BeginPlay: it is only needed once, and besides, the cast to PlayerController will fail for new spawned BP_Player instances. We simply use this already set mapping with Posses in the BP_PlayerGameMode. ANYTHING executed beyond this node wouldn't be executed after the first respawn!
  (Input|AddMappingContext))

(event Game|Damage|EventAnyDamage
  (params (Damage :type Float%20%28single-precision%29) (DamageType :type Damage%20Type%20Object%20Reference) (InstigatedBy :type Controller%20Object%20Reference) (DamageCauser :type Actor%20Object%20Reference))
  ;[1 1 1] Damage
  (|CallParentFunction Damage DamageType InstigatedBy DamageCauser)
  (CallFunction|StopDash)
  (Variables|Shoot|SetHasBeenDamagedWhileCharging true)
  (CallFunction|SetInvincible)
  (CallFunction|Knockback DamageCauser)
  (|DisableInputForDuration (Variables|Damage|GetReactingToHitDuration)))

(event EventTick
  (params (DeltaSeconds :type Float%20%28single-precision%29))
  ;[1 1 1] Wall Sliding
  (|CallParentFunction 0.0)
  (if (|CanWallSlide)
    (bind _wallhit (|PerformLineTraceAgainstWall))
    (bind _output_get (Variables|WallSlide|SetIsWallSliding _wallhit))
    (if _output_get
      (|ClampFallVelocityForWallSliding)
      (else
        (|ResetFallVelocityToDefault)))
    (else
      (Variables|WallSlide|SetIsWallSliding false))))

(fn ConstructionScript
  (|CallParentFunction))

(fn RotateXDirection
  (params (Direction :type Float%20%28double-precision%29))
  (if (not (Variables|Dash|GetIsDashing))
    (Pawn|SetControlRotation (Pawn|GetController) (Math|Rotator|SelectRotator (Math|Rotator|MakeRotator 0.0 0.0 0.0) (Math|Rotator|MakeRotator 0.0 0.0 1.8e+02) (>= Direction 0.0)))))

(fn SpawnBullet
  (params (ProjectileClass :type BP%20Projectile%20Player%20BASE%20Class%20Reference))
  (bind _self self)
  (bind _bulletspawn (Variables|Default|GetBulletSpawn))
  (bind _projectilescost (Variables|Shoot|Energy|GetProjectilesCost))
  (bind _iswallsliding (Variables|WallSlide|GetIsWallSliding))
  (bind _bulletspawn_wallsliding (Variables|Default|GetBulletSpawn_WallSliding))
  (bind (_value _returnvalue) (Utilities|Map|Find _projectilescost ProjectileClass))
  (bind _returnvalue_2 (select _iswallsliding _bulletspawn_wallsliding _bulletspawn))
  (if _returnvalue
    (LocalVariables|SetProjectileToSpawnCost _value)
    (if (>= (Variables|Default|GetBulletEnergy) (LocalVariables|GetProjectileToSpawnCost))
      (bind _returnvalue_3 (Game|SpawnActorfromClass ProjectileClass (Math|Transform|MakeTransform (Transformation|GetWorldLocation _returnvalue_2) (Transformation|GetWorldRotation _returnvalue_2) "1.000000,1.000000,1.000000") "AlwaysSpawn" "MultiplyWithRoot" _self _self))
      (Variables|/Game/Blueprints/Projectiles/BP_Projectile_BASE.BP_Projectile_BASE_C|SetDamage _returnvalue_3 (LocalVariables|GetProjectileToSpawnCost))
      (Collision|SetCollisionEnabled (Variables|/Game/Blueprints/Projectiles/BP_Projectile_BASE.BP_Projectile_BASE_C|GetSphere _returnvalue_3) "QueryAndPhysics")
      (return _returnvalue_3)
      (else
        (return 0)))
    (else
      (Development|PrintString (Utilities|String|Append "Cost not found for projectile: " (Utilities|GetClassDisplayName ProjectileClass)) true true "(R=0.666667,G=0.010044,B=0.000000,A=1.000000)" 1e+01 "SpawnBullet"))))

(fn ToggleSpriteVisibility
  (Rendering|ToggleVisibility (Variables|Default|GetSprite) false))

(fn ConsumeEnergyfromProjectile
  (params (Projectile :type BP%20Projectile%20Player%20BASE%20Object%20Reference))
  (Variables|Default|SetBulletEnergy (- (Variables|Default|GetBulletEnergy) (Variables|/Game/Blueprints/Projectiles/BP_Projectile_BASE.BP_Projectile_BASE_C|GetDamage Projectile))))

(fn HandleChargingFlash
  (params (ElapsedTime :type Float%20%28double-precision%29))
  (if (Variables|Shoot|GetHasBeenDamagedWhileCharging)
    (Variables|Shoot|SetHasBeenDamagedWhileCharging false)
    (elif (not (< ElapsedTime (Variables|Shoot|Energy|GetPartialChargeThreshold)))
      (if (< ElapsedTime (Variables|Shoot|Energy|GetFullChargeThreshold))
        (if (not (Variables|Flash|PartialCharge|GetPartialChargeAlreadyFlashed))
          (Variables|Flash|PartialCharge|SetPartialChargeAlreadyFlashed true)
          (CallFunction|Flash (Variables|Flash|PartialCharge|GetPartialChargeFlashIntensity) (Variables|Flash|PartialCharge|GetPartialChargeFlashPlayRate) (Variables|Flash|PartialCharge|GetPartialChargeFlashColor)))
        (elif (not (Variables|Flash|FullCharge|GetFullChargeAlreadyFlashed))
          (Variables|Flash|FullCharge|SetFullChargeAlreadyFlashed true)
          (CallFunction|Flash (Variables|Flash|FullCharge|GetFullChargeFlashIntensity) (Variables|Flash|FullCharge|GetFullChargeFlashPlayRate) (Variables|Flash|FullCharge|GetFullChargeFlashColor)))))))

(fn StopDash
  (Audio|Components|Audio|Stop (Variables|Default|GetDashTimeline))
  (CallFunction|ModifyCapsuleStartDash 1)
  (Variables|Dash|SetIsDashing false)
  (Variables|Dash|SetDashDirection 0.0))

(fn ApplyDamageifEnemy
  (params (Actor :type Actor%20Object%20Reference) (ActorComponent :type Actor%20Component%20Object%20Reference))
  (bind _asbp_enemy_base (Utilities|Casting|CastToBP_Enemy_BASE Actor))
  (if (== (Variables|/Script/Engine.Character|GetCapsuleComponent _asbp_enemy_base) ActorComponent)
    (Game|Damage|ApplyDamage self 1.0 0 Actor)
    (return)))

(fn ModifyCapsuleStartDash
  (params (IncreaseOrDecrease :type Integer))
  (bind _capsulecomponent (Variables|Default|GetCapsuleComponent))
  (bind _result (Utilities|NegateInt IncreaseOrDecrease)
    (:%20%20
      (Components|Capsule|SetCapsuleHalfHeight _capsulecomponent (- (Variables|/Script/Engine.CapsuleComponent|GetCapsuleHalfHeight _capsulecomponent) (* (Variables|Dash|GetDashCapsuleDelta) _result)) false)
      (Transformation|AddWorldOffset (Variables|Default|GetSprite) (Math|Vector|MakeVector 0.0 0.0 (* (Variables|Dash|GetDashCapsuleDelta) _result)) false true)
      (Transformation|AddWorldOffset (Variables|Default|GetSpringArm) (Math|Vector|MakeVector 0.0 0.0 (* (Variables|Dash|GetDashCapsuleDelta) _result)) false true))))