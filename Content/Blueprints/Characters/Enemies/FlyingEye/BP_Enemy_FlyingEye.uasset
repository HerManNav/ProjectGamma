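; Flying eye enemy that detects the player and provides movement and turning functions.
; An aggro sphere, sized in the construction script from AggroRadius, stores the player on overlap and signals in-range or out-of-sight.
; Each tick it traces to the player against static world objects, using paired DoOnce gates to signal only when line of sight changes.
; MoveTo applies movement input scaled by ChasingSpeed, while TurnTo and TurnAround rotate the actor.
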(event OnComponentBeginOverlap(AggroSphere)
  (params (OverlappedComponent :type Primitive%20Component%20Object%20Reference) (OtherActor :type Actor%20Object%20Reference) (OtherComp :type Primitive%20Component%20Object%20Reference) (OtherBodyIndex :type Integer) (bFromSweep :type Boolean) (SweepResult :type Hit%20Result%20Structure%20%28by%20ref%29))
  (bind _asbp_player (Utilities|Casting|CastToBP_Player OtherActor))
  (bind _output_get (Variables|Chasing|SetPlayer _asbp_player))
  (Default|CallPlayerGotinRange _output_get))

(event OnComponentEndOverlap(AggroSphere)
  (params (OverlappedComponent :type Primitive%20Component%20Object%20Reference) (OtherActor :type Actor%20Object%20Reference) (OtherComp :type Primitive%20Component%20Object%20Reference) (OtherBodyIndex :type Integer))
  (Utilities|Casting|CastToBP_Player OtherActor)
  (Variables|Chasing|SetPlayer 0)
  (Default|CallPlayerGotOutSight))

(event EventBeginPlay
  (|CallParentFunction)
  (Development|SetHiddeninGame (Variables|Default|GetAggroSphere) (not (Variables|Default|GetbShowDebugCapsules)) false))

(event EventTick
  (params (DeltaSeconds :type Float%20%28single-precision%29))
  (|CallParentFunction DeltaSeconds)
  (bind _player (Variables|Chasing|GetPlayer)
    (:then
      (bind _returnvalue (Collision|LineTraceForObjects (Transformation|GetActorLocation) (Transformation|GetActorLocation _player) (Utilities|Array|MakeArray "ObjectTypeQuery1") false 0 (Variables|Default|GetbShowDebugTraces)))
      (if _returnvalue
        (Utilities|FlowControl|DoOnce false :!label _label
          (:Completed
            (Default|CallPlayerGotOutSight)
            (goto _label_2 Reset)))
        (else
          (Utilities|FlowControl|DoOnce false :!label _label_2
            (:Completed
              (Default|CallPlayerGotinRange _player)
              (goto _label Reset))))))
    (:else)))

(fn ConstructionScript
  (|CallParentFunction)
  (Components|Sphere|SetSphereRadius (Variables|Default|GetAggroSphere) (Variables|Chasing|GetAggroRadius) true))

(fn Turnto
  (params (Rotation :type Rotator))
  (Transformation|SetActorRotation Rotation))

(fn Moveto
  (params (Position :type Vector))
  (Pawn|Input|AddMovementInput Position (Variables|Chasing|GetChasingSpeed) false))

(fn TurnAround
  (Class|Actor|AddActorWorldRotation "0.000000,180.000000,0.000000"))