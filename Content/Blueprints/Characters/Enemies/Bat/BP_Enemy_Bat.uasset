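; Bat enemy Blueprint that flies between two placed points, Position1 and Position2.
; BeginPlay caches both world locations, sets the timeline play rate from MovementSpeed, then spawns and possesses with its default AI controller, so Auto Possess AI must be disabled.
; MoveForward and MoveBackward play the timeline forward or in reverse, lerping the actor's location without sweep.
; The timeline calls FinishedMovement when a move completes.
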(event Custom|MoveForward
  (bind _alpha (Timeline|BatMovementTimeline PlayFromStart)
    (:Update
      (Transformation|SetActorLocation (Math|Vector|Lerp(Vector) (Variables|Drifting|GetPosition1Location) (Variables|Drifting|GetPosition2Location) _alpha) false false))
    (:Finished
      (Default|CallFinishedMovement))))

(event Custom|MoveBackward
  (bind _alpha (Timeline|BatMovementTimeline ReverseFromEnd)
    (:Update
      (Transformation|SetActorLocation (Math|Vector|Lerp(Vector) (Variables|Drifting|GetPosition1Location) (Variables|Drifting|GetPosition2Location) _alpha) false false))
    (:Finished
      (Default|CallFinishedMovement))))

(event EventBeginPlay
  (|CallParentFunction)
  (Utilities|FlowControl|Sequence
    (:then_0
      (Components|Timeline|SetPlayRate (Variables|Default|GetBatMovementTimeline) (Variables|Drifting|GetMovementSpeed)))
    (:then_1
      (Variables|Drifting|SetPosition1Location (Transformation|GetWorldLocation (Variables|Default|GetPosition1)))
      (Variables|Drifting|SetPosition2Location (Transformation|GetWorldLocation (Variables|Default|GetPosition2))))
    (:then_2
      (Pawn|SpawnDefaultController) ; "Auto possess AI" should be disabled!
      (Pawn|Possess (AI|GetAIController self) self))))

(fn ConstructionScript
  (|CallParentFunction))