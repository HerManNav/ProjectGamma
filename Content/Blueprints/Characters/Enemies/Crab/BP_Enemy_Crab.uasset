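; Crab enemy for a 2D flipbook-based game that detects ledges in front of it as it walks.
; MoveAhead adds movement input along the forward X axis and switches the sprite to the walk flipbook.
; Each Tick, until HasReachedEndOfDirection is set, a WorldStatic line trace drops from foot level just beyond the capsule.
; A missed trace sets that flag; the turnaround itself is not handled in this graph.
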(event Custom|MoveAhead
  (params (Amount :type Float%20%28double-precision%29))
  (Pawn|Input|AddMovementInput (Math|Vector|MakeVector (.x (Transformation|GetActorForwardVector)) 0.0 0.0) Amount false)
  (Sprite|SetFlipbook (Variables|Default|GetSprite) "/Game/PaperAssets/Characters/Enemies/crab/crab__Walk.crab__Walk"))

(event EventTick
  (params (DeltaSeconds :type Float%20%28single-precision%29))
  (bind _returnvalue (Transformation|GetActorLocation))
  (bind _returnvalue_2 (Transformation|GetActorForwardVector))
  (bind _distanceforturningback (Variables|Movement|GetDistanceForTurningBack))
  (bind _capsulecomponent (Variables|Default|GetCapsuleComponent))
  (bind _capsuleradius (Variables|/Script/Engine.CapsuleComponent|GetCapsuleRadius _capsulecomponent))
  (bind _capsulehalfheight (Variables|/Script/Engine.CapsuleComponent|GetCapsuleHalfHeight _capsulecomponent))
  (bind _returnvalue_3 (* _capsulehalfheight -1.0))
  (bind _returnvalue_4 (+ _capsuleradius _distanceforturningback))
  (bind _returnvalue_5 (* _returnvalue_4 (.x _returnvalue_2)))
  (bind _returnvalue_6 (+ _returnvalue (Math|Vector|MakeVector _returnvalue_5 0.0 _returnvalue_3)))
  (if (not (Variables|Movement|GetbHasReachedEndOfDirection))
    (bind _returnvalue_7 (Collision|LineTraceForObjects _returnvalue_6 (- _returnvalue_6 (Math|Vector|MakeVector 0.0 0.0 (Variables|Movement|GetFallTracingLength))) (Utilities|Array|MakeArray "ObjectTypeQuery1") false 0 "None"))
    (Variables|Movement|SetbHasReachedEndOfDirection (not _returnvalue_7))))

(fn ConstructionScript
  (|CallParentFunction))