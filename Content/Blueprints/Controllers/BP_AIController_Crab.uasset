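; AI controller for the crab enemy that drives a back-and-forth patrol.
; It caches the possessed BP_Enemy_Crab, then on Tick moves it ahead until the pawn flags the end of its direction.
; A DoOnce then switches the flipbook to idle, pauses briefly, turns the crab around and clears the flag.
; The DoOnce resets while the crab moves, so each turn triggers only once.
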(event EventTick
  (params (DeltaSeconds :type Float%20%28single-precision%29))
  (bind _bpcrab (Variables|Default|GetBPCrab))
  (bind _bpcrab_2 (Variables|Default|GetBPCrab))
  (if (not (Variables|/Game/Blueprints/Characters/Enemies/BP_Enemy_Crab.BP_Enemy_Crab_C|GetbHasReachedEndOfDirection _bpcrab))
    (Default|MoveAhead _bpcrab 1.0)
    (goto _label Reset)
    (else
      (Utilities|FlowControl|DoOnce false :!label _label
        (:Completed
          (Sprite|SetFlipbook (Variables|/Script/Paper2D.PaperCharacter|GetSprite (Variables|Default|GetBPCrab)) "/Game/PaperAssets/Characters/Enemies/crab/crab__Idle.crab__Idle")
          (Utilities|FlowControl|Delay 2.0)
          (Class|Actor|AddActorWorldRotation _bpcrab_2 "0.000000,180.000000,0.000000")
          (Variables|/Game/Blueprints/Characters/Enemies/BP_Enemy_Crab.BP_Enemy_Crab_C|SetbHasReachedEndOfDirection _bpcrab_2 false))))))

(event EventPossess
  (params (PossessedPawn :type Pawn%20Object%20Reference))
  (bind _asbp_enemy_crab (Utilities|Casting|CastToBP_Enemy_Crab PossessedPawn))
  (Variables|Default|SetBPCrab _asbp_enemy_crab))

(fn ConstructionScript
  (|CallParentFunction))