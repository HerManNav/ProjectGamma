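; AI controller for the bat enemy that runs its back-and-forth patrol.
; On possess, it stores the BP_Enemy_Bat pawn, binds to its FinishedMovement event and starts it moving forward.
; Each finished movement triggers a random wait between the bat's min and max patrol waiting times, then a FlipFlop alternates backward and forward moves, so the patrol loops.
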(event Custom|GoForNextPatrolRound
  (bind _bpbat (Variables|Default|GetBPBat))
  (bind _bpbat_2 (Variables|Default|GetBPBat))
  (Utilities|FlowControl|Delay (Math|Random|RandomFloatinRange (Variables|/Game/Blueprints/Characters/Enemies/Bat/BP_Enemy_Bat.BP_Enemy_Bat_C|GetMinPatrolWaitingTime _bpbat) (Variables|/Game/Blueprints/Characters/Enemies/Bat/BP_Enemy_Bat.BP_Enemy_Bat_C|GetMaxPatrolWaitingTime _bpbat)))
  (Utilities|FlowControl|FlipFlop
    (:A
      (Default|MoveBackward _bpbat_2))
    (:B
      (Default|MoveForward _bpbat_2))))

(event EventPossess
  (params (PossessedPawn :type Pawn%20Object%20Reference))
  (bind _asbp_enemy_bat (Utilities|Casting|CastToBP_Enemy_Bat PossessedPawn))
  (bind _output_get (Variables|Default|SetBPBat _asbp_enemy_bat))
  (EventDispatchers|BindEventtoFinishedMovement _output_get (delegate Custom|GoForNextPatrolRound)) ; Suscribe to BPBat's FinishedMovement event
  (Default|MoveForward _output_get))

(fn ConstructionScript
  (|CallParentFunction))