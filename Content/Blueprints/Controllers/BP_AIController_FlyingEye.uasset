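; AI controller for the flying eye enemy that makes it chase and face the player.
; On possess it binds to the enemy's range events, storing the player when in range and clearing it when out of range.
; While a player is stored, each tick passes the normalized direction to the player into the enemy's MoveToPosition and turns it with a look-at rotation.
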(event Custom|PlayerSeen
  (params (Player :type BP%20Player%20Object%20Reference))
  (Variables|Default|SetPlayer Player))

(event Custom|PlayerOutOfSight
  (Variables|Default|SetPlayer 0))

(event EventTick
  (params (DeltaSeconds :type Float%20%28single-precision%29))
  (bind _bpflyingeye (Variables|Default|GetBPFlyingEye))
  (|CallParentFunction DeltaSeconds)
  (bind _player (Variables|Default|GetPlayer)
    (:then
      (Default|MovetoPosition _bpflyingeye (Math|Vector|Normalize (- (Transformation|GetActorLocation _player) (Transformation|GetActorLocation _bpflyingeye))))
      (Default|Turnto _bpflyingeye (Math|Rotator|FindLookatRotation (Transformation|GetActorLocation _bpflyingeye) (Transformation|GetActorLocation _player))))
    (:else)))

(event EventPossess
  (params (PossessedPawn :type Pawn%20Object%20Reference))
  (bind _asbp_enemy_flying_eye (Utilities|Casting|CastToBP_Enemy_FlyingEye PossessedPawn))
  (bind _output_get (Variables|Default|SetBPFlyingEye _asbp_enemy_flying_eye))
  (Utilities|FlowControl|Sequence
    (:then_0
      (EventDispatchers|BindEventtoPlayerGotinRange _output_get (delegate Custom|PlayerSeen)))
    (:then_1
      (EventDispatchers|BindEventtoPlayerGotOutRange _output_get (delegate Custom|PlayerOutOfSight)))))

(fn ConstructionScript
  (|CallParentFunction))