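; AI controller for the Lizard that makes its possessed pawn fire repeatedly at random intervals.
; On possess, it casts the pawn to BP_Lizard and caches the reference.
; Tick feeds a Delay randomized between the min and max shot times, which ignores re-triggers while pending and then calls Shoot on the Lizard.
; It contains no targeting or movement logic.
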(event EventTick
  (params (DeltaSeconds :type Float%20%28single-precision%29))
  (|CallParentFunction DeltaSeconds)
  (Utilities|FlowControl|Delay (Math|Random|RandomFloatinRange (Variables|Shooting|GetMinTimeBetweenShots) (Variables|Shooting|GetMaxTimeBetweenShots)))
  (Default|Shoot (Variables|Default|GetAs%20BP%20Lizard)))

(event EventPossess
  (params (PossessedPawn :type Pawn%20Object%20Reference))
  (|CallParentFunction PossessedPawn)
  (bind _asbp_lizard (Utilities|Casting|CastToBP_Lizard PossessedPawn))
  (Variables|Default|SetAs%20BP%20Lizard _asbp_lizard))

(fn ConstructionScript
  (|CallParentFunction))