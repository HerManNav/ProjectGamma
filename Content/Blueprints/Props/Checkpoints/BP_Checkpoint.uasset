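; BP_Checkpoint is a checkpoint prop that registers itself with BP_PlayerGameMode when the player overlaps its collision box.
; It caches the game mode on BeginPlay, then sets that mode's CheckPoint to itself and turns its cube blue.
; A DoOnce ahead of the BP_Player cast means the first overlap by any actor uses up the trigger.
; Debug strings print on overlap.
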(event OnComponentBeginOverlap(CollisionBox)
  (params (OverlappedComponent :type Primitive%20Component%20Object%20Reference) (OtherActor :type Actor%20Object%20Reference) (OtherComp :type Primitive%20Component%20Object%20Reference) (OtherBodyIndex :type Integer) (bFromSweep :type Boolean) (SweepResult :type Hit%20Result%20Structure%20%28by%20ref%29))
  (Development|PrintString "hey")
  (Utilities|FlowControl|DoOnce false
    (:Completed
      (Development|PrintString "Hello")
      (Utilities|Casting|CastToBP_Player OtherActor)
      (Variables|/Game/Blueprints/BP_PlayerGameMode.BP_PlayerGameMode_C|SetCheckPoint (Variables|Default|GetGameMode) self)
      (Rendering|Material|SetMaterial (Variables|Default|GetCube) 0 "/AnimationSharing/AnimSharingBlue.AnimSharingBlue"))))

(event EventBeginPlay
  (bind _asbp_player_game_mode (Utilities|Casting|CastToBP_PlayerGameMode (Game|GetGameMode)))
  (Variables|Default|SetGameMode _asbp_player_game_mode))

(fn ConstructionScript)